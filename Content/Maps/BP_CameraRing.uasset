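; BP_CameraRing is a camera rig whose spring arm slowly orbits by adding yaw each tick at SpeedCamera.
; ZoomIn stops the orbit, stores the current rotation, and plays a timeline that blends the arm to a fixed yaw, steeper pitch, shorter length and offset position.
; ZoomOut restores the orbit speed and reverses that timeline from the end, while yaw keeps being driven from the stored rotation.
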(event Custom|Zoom%20In
  (bind _springarm (Variables|Default|GetSpringArm))
  (Variables|Default|SetSpeedCamera 0.0)
  (Variables|Default|SetOldRot (Variables|/Script/Engine.SceneComponent|GetRelativeRotation (Variables|Default|GetSpringArm)))
  (bind _newtrack_0 (Timeline|ZoomInTimeline PlayFromStart)
    (:Update
      (Transformation|SetRelativeRotation (Variables|Default|GetSpringArm) (Math|Rotator|MakeRotator 0.0 (Math|Float|Lerp -2e+01 -4e+01 _newtrack_0) (Math|Float|Lerp (.Yaw (Math|Rotator|BreakRotator (Variables|Default|GetOldRot))) 135.0 _newtrack_0)) false false)
      (Variables|/Script/Engine.SpringArmComponent|SetTargetArmLength _springarm (Math|Float|Lerp 1.5e+03 6.5e+02 _newtrack_0))
      (Transformation|SetRelativeLocation _springarm (Math|Vector|Lerp(Vector) "0, 0, 0" "200.000000,-200.000000,0.000000" _newtrack_0) false false))))

(event Custom|Zoom%20Out
  (bind _springarm (Variables|Default|GetSpringArm))
  (Variables|Default|SetSpeedCamera 1e+01)
  (bind _newtrack_0 (Timeline|ZoomInTimeline ReverseFromEnd)
    (:Update
      (Transformation|SetRelativeRotation (Variables|Default|GetSpringArm) (Math|Rotator|MakeRotator 0.0 (Math|Float|Lerp -2e+01 -4e+01 _newtrack_0) (Math|Float|Lerp (.Yaw (Math|Rotator|BreakRotator (Variables|Default|GetOldRot))) 135.0 _newtrack_0)) false false)
      (Variables|/Script/Engine.SpringArmComponent|SetTargetArmLength _springarm (Math|Float|Lerp 1.5e+03 6.5e+02 _newtrack_0))
      (Transformation|SetRelativeLocation _springarm (Math|Vector|Lerp(Vector) "0, 0, 0" "200.000000,-200.000000,0.000000" _newtrack_0) false false))))

(event EventBeginPlay)

(event Collision|EventActorBeginOverlap
  (params (OtherActor :type Actor%20Object%20Reference)))

(event EventTick
  (params (DeltaSeconds :type Float%20%28single-precision%29))
  (Transformation|AddRelativeRotation (Variables|Default|GetSpringArm) (Math|Rotator|MakeRotator 0.0 0.0 (* DeltaSeconds (Variables|Default|GetSpeedCamera))) false false))

(fn ConstructionScript)