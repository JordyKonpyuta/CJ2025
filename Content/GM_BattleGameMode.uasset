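; Battle game mode that runs a tournament of automatic two-versus-two fights between furniture units (BP_Meuble) against a shuffled list of trainers.
; Each battle spawns the enemy pair from data tables and the player's pair via PrepareBattleEnd, then loops timed turns in speed order.
; Attacks resolve targets by side and left/right slot before applying damage, heal, buff or debuff effects.
; Results accumulate per battle until the tournament ends, reports victories and saves.
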(event Custom|GetRidOfAllMeubles
  ;[0.15 0.15 0.15 0.5] Remove all Meubles
  (bind _outactors (Actor|GetAllActorsOfClass "/Game/Furniture/BP_Meuble.BP_Meuble_C"))
  (for _array_element _outactors
    (Default|TakeDamage _array_element 10000))
  (Utilities|Array|Clear (Variables|TousLesMeubles|GetToutLesMeublesJoueur))
  (Utilities|Array|Clear (Variables|TousLesMeubles|GetTousLesMeublesEnnemis))
  (Utilities|Array|Clear (Variables|TousLesMeubles|GetTousLesMeublesParOrdreDeVitesse)))

(event Custom|PrepareBattleStart
  (bind _all_trainers_to_fight (Variables|Trainers|GetAll%20Trainers%20to%20Fight))
  (bind _all_trainers_to_fight_2 (Variables|Trainers|GetAll%20Trainers%20to%20Fight))
  (bind _output (Utilities|Array|Get(acopy) _all_trainers_to_fight))
  (bind _output_2 (Utilities|Array|Get(acopy) _all_trainers_to_fight_2))
  (bind (_meuble1 _sequenceactions1) (Utilities|Struct|BreakStruct_TrainerData _output))
  (bind (_meuble2 _sequenceactions2) (Utilities|Struct|BreakStruct_TrainerData _output_2))
  (bind (_datatable _rowname) (Utilities|Struct|BreakDataTableRowHandle _meuble1))
  (bind (_datatable_2 _rowname_2) (Utilities|Struct|BreakDataTableRowHandle _meuble2))
  ;[0 1 0.5441 0.5 60] PREPARER LES COMBATS - INITIALISATION : ENNEMIS
  (Utilities|FlowControl|Sequence
    (:then_0
      (bind _returnvalue (Game|SpawnActorfromClass "/Game/Furniture/BP_Meuble.BP_Meuble_C" (Math|Transform|MakeTransform "-150.000000,150.000000,100.000000") "Undefined" "MultiplyWithRoot" 0 0))
      (Utilities|Array|Add (Variables|TousLesMeubles|GetTousLesMeublesEnnemis) _returnvalue)
      (bind _returnvalue_2 (Utilities|GetDataTableRow _datatable _rowname)
        (:then
          (Default|CustomBeginPlay _returnvalue _returnvalue_2)
          (Utilities|Array|Add (Variables|TousLesMeublesData|GetMeublesEnnemis) _returnvalue_2)
          (Variables|/Game/Furniture/BP_Meuble.BP_Meuble_C|SetAGaucheEnCombat _returnvalue true)
          (Variables|/Game/Furniture/BP_Meuble.BP_Meuble_C|SetOrdreDesAttaques _returnvalue _sequenceactions1)
          (Variables|/Game/Furniture/BP_Meuble.BP_Meuble_C|SetGamemodeRef _returnvalue self)
          (Variables|/Game/Furniture/BP_Meuble.BP_Meuble_C|SetCameraRef _returnvalue (Variables|Ref|GetCameraRef)))
        (:RowNotFound
          (CallFunction|HandlingErrors))))
    (:then_1
      (bind _returnvalue_3 (Game|SpawnActorfromClass "/Game/Furniture/BP_Meuble.BP_Meuble_C" (Math|Transform|MakeTransform "-150.000000,-150.000000,100.000000") "Undefined" "MultiplyWithRoot" 0 0))
      (Utilities|Array|Add (Variables|TousLesMeubles|GetTousLesMeublesEnnemis) _returnvalue_3)
      (bind _returnvalue_4 (Utilities|GetDataTableRow _datatable_2 _rowname_2)
        (:then
          (Default|CustomBeginPlay _returnvalue_3 _returnvalue_4)
          (Utilities|Array|Add :TargetArray (Variables|TousLesMeublesData|GetMeublesEnnemis))
          (Variables|/Game/Furniture/BP_Meuble.BP_Meuble_C|SetOrdreDesAttaques _returnvalue_3 _sequenceactions2)
          (Variables|/Game/Furniture/BP_Meuble.BP_Meuble_C|SetGamemodeRef _returnvalue_3 self)
          (Variables|/Game/Furniture/BP_Meuble.BP_Meuble_C|SetCameraRef _returnvalue_3 (Variables|Ref|GetCameraRef)))
        (:RowNotFound
          (CallFunction|HandlingErrors))))))

(event Custom|IsATeamDead
  (if (Utilities|Array|IsEmpty (Variables|TousLesMeubles|GetTousLesMeublesEnnemis))
    (CallFunction|EndOfBattle true)
    (elif (Utilities|Array|IsEmpty (Variables|TousLesMeubles|GetToutLesMeublesJoueur))
      (CallFunction|EndOfBattle false)
      (else
        (CallFunction|BattleLoop)))))

(event Custom|BattleLoopBegins
  (CallFunction|OrderCharactersbySpeed)
  (Utilities|FlowControl|Delay 1.0)
  (CallFunction|BattleLoop))

(event Custom|EndOfBattle
  (params (PlayerVictory :type Boolean))
  (bind _all_trainers_to_fight (Variables|Trainers|GetAll%20Trainers%20to%20Fight))
  (bind _victorystream (Variables|TournamentResults|GetVictoryStream))
  (bind _curbattle (Variables|TournamentResults|GetCurBattle))
  ;[0 1 0.9782 0.5 36] BATTLE END
  (Default|ZoomOut (Variables|Ref|GetCameraRef))
  (if PlayerVictory
    (Math|Integer|IncrementInt (Variables|TournamentResults|GetVictories)
      (:%20%20
        (Utilities|Array|SetArrayElem _victorystream _curbattle true true)))
    (else
      (Utilities|Array|SetArrayElem _victorystream _curbattle false true)))
  (CallFunction|GetRidOfAllMeubles)
  (Utilities|Array|RemoveIndex _all_trainers_to_fight)
  (Math|Integer|IncrementInt (Variables|TournamentResults|GetCurBattle)
    (:%20%20
      (if (Utilities|Array|IsEmpty _all_trainers_to_fight)
        (CallFunction|EndOfTournament)
        (else
          (Widget|RemovefromParent (Variables|Ref|GetBattleWidgetRef))
          (UserInterface|Viewport|AddtoViewport (Variables|Ref|GetBeforeCombatWidgetRef) 0)
          (CallFunction|PrepareBattleStart))))))

(event Custom|EndOfTournament
  ;[0.15 0.1183 0 0.5 46] AJOUTER LA TP A UNE AUTRE MAP
  (Default|TournoiTermine (Variables|Ref|GetGameInstanceRef) (Variables|TournamentResults|GetVictories))
  (Utilities|FlowControl|Delay 1.0)
  (bind _returnvalue (UserInterface|CreateWidget "/Game/UI/WBP_TournoiEnd.WBP_TournoiEnd_C"))
  (UserInterface|Viewport|AddtoViewport _returnvalue 0)
  (Default|SaveGame (Variables|Ref|GetGameInstanceRef)))

(event Custom|BattleLoop
  (bind _touslesmeublesparordredevitesse (Variables|TousLesMeubles|GetTousLesMeublesParOrdreDeVitesse))
  (bind _output (Utilities|Array|Get(acopy) _touslesmeublesparordredevitesse))
  (if (Utilities|Array|IsNotEmpty _touslesmeublesparordredevitesse)
    (CallFunction|Attaque _output)
    (Utilities|Array|RemoveItem _touslesmeublesparordredevitesse _output)
    (Utilities|FlowControl|Delay 1.0)
    (CallFunction|IsATeamDead)
    (else
      (CallFunction|BattleLoopBegins))))

(event Custom|HandlingErrors
  ;[2 0 0 1 124] ERROR
  (Development|PrintString "Error in the Battle Gamemode!" false true "(R=0.000000,G=0.660000,B=1.000000,A=1.000000)" 1e+03))

(event Custom|PrepareBattleEnd
  (params (Fourniture_BaseData :type Array%20of%20Struct%20Furniture%20Data%20Structures) (Meuble1ActionsSequence :type Array%20of%20Integers) (Meuble2ActionsSequence :type Array%20of%20Integers))
  ;[0 1 0.1772 0.5 60] FIN DE PREPARATION DE COMBATS - INITIALISATION : JOUEUR
  (Variables|TousLesMeublesData|SetMeublesJoueurs Fourniture_BaseData)
  (Utilities|FlowControl|Sequence
    (:then_0
      (bind _returnvalue (Game|SpawnActorfromClass "/Game/Furniture/BP_Meuble.BP_Meuble_C" (Math|Transform|MakeTransform "150.000000,150.000000,100.000000" "0.000000,180.000000,0.000000") "Undefined" "MultiplyWithRoot" 0 0))
      (Utilities|Array|Add (Variables|TousLesMeubles|GetToutLesMeublesJoueur) _returnvalue)
      (Default|CustomBeginPlay _returnvalue (Utilities|Array|Get(acopy) (Variables|TousLesMeublesData|GetMeublesJoueurs)))
      (Variables|/Game/Furniture/BP_Meuble.BP_Meuble_C|SetAGaucheEnCombat _returnvalue true)
      (Variables|/Game/Furniture/BP_Meuble.BP_Meuble_C|SetOrdreDesAttaques _returnvalue Meuble1ActionsSequence)
      (Variables|/Game/Furniture/BP_Meuble.BP_Meuble_C|SetGamemodeRef _returnvalue self)
      (Variables|/Game/Furniture/BP_Meuble.BP_Meuble_C|SetCameraRef _returnvalue (Variables|Ref|GetCameraRef)))
    (:then_1
      (bind _returnvalue_2 (Game|SpawnActorfromClass "/Game/Furniture/BP_Meuble.BP_Meuble_C" (Math|Transform|MakeTransform "150.000000,-150.000000,100.000000" "0.000000,180.000000,0.000000") "Undefined" "MultiplyWithRoot" 0 0))
      (Utilities|Array|Add (Variables|TousLesMeubles|GetToutLesMeublesJoueur) _returnvalue_2)
      (Default|CustomBeginPlay _returnvalue_2 (Utilities|Array|Get(acopy) (Variables|TousLesMeublesData|GetMeublesJoueurs) 1))
      (Variables|/Game/Furniture/BP_Meuble.BP_Meuble_C|SetOrdreDesAttaques _returnvalue_2 Meuble2ActionsSequence)
      (Variables|/Game/Furniture/BP_Meuble.BP_Meuble_C|SetGamemodeRef _returnvalue_2 self)
      (Variables|/Game/Furniture/BP_Meuble.BP_Meuble_C|SetCameraRef _returnvalue_2 (Variables|Ref|GetCameraRef)))
    (:then_2
      (CallFunction|SeeFight))))

(event Custom|SeeFight
  ;[0.15 0.03906 0.03906 0.5 32] A développer - jouer avec la caméra pour la faire se rapprocher
  (CallFunction|BattleLoopBegins)
  (Default|Zoomin (Variables|Ref|GetCameraRef))
  (bind _returnvalue (UserInterface|CreateWidget "/Game/UI/WBP_Combat.WBP_Combat_C"))
  (bind _output_get (Variables|Ref|SetBattleWidgetRef _returnvalue))
  (UserInterface|Viewport|AddtoViewport _output_get 0))

(event Custom|DeadMeuble
  (params (DeadMeuble :type BP%20Meuble%20Object%20Reference%20%28by%20ref%29))
  ;[0.15 0.15 0.15 0.5] Dead Meuble
  (if (Utilities|Array|ContainsItem (Variables|TousLesMeubles|GetToutLesMeublesJoueur) DeadMeuble)
    (Utilities|Array|RemoveItem (Variables|TousLesMeubles|GetToutLesMeublesJoueur) DeadMeuble)
    (else
      (Utilities|Array|RemoveItem (Variables|TousLesMeubles|GetTousLesMeublesEnnemis) DeadMeuble)))
  (Utilities|Array|RemoveItem (Variables|TousLesMeubles|GetTousLesMeublesParOrdreDeVitesse) DeadMeuble))

(event EventBeginPlay
  ;[0.9896 0.9792 1 0.5 72] INITIALISER LE TOURNOI
  (bind _asgi_main_game_instance (Utilities|Casting|CastToGI_MainGameInstance (Game|GetGameInstance)))
  (bind _output_get (Variables|Ref|SetGameInstanceRef _asgi_main_game_instance))
  (bind _alltrainerstofight (Default|InitTournament _output_get))
  (bind _output_get_2 (Variables|Trainers|SetAll%20Trainers%20to%20Fight _alltrainerstofight))
  (Utilities|Array|Shuffle _output_get_2)
  (CallFunction|PrepareBattleStart)
  (bind _returnvalue (Actor|GetActorOfClass "/Game/Maps/BP_CameraRing.BP_CameraRing_C"))
  (bind _output_get_3 (Variables|Ref|SetCameraRef _returnvalue))
  (Game|Player|SetViewTargetwithBlend (Game|GetPlayerController 0) _output_get_3 0.0 "VTBlend_Linear" 0.0 false)
  (bind _returnvalue_2 (UserInterface|CreateWidget "/Game/UI/WBP_BeforeCombat.WBP_BeforeCombat_C"))
  (bind _output_get_4 (Variables|Ref|SetBeforeCombatWidgetRef _returnvalue_2))
  (UserInterface|Viewport|AddtoViewport _output_get_4 0))

(fn ConstructionScript)

(fn OrderCharactersbySpeed
  (bind _touslesmeublestoutcourt (LocalVariables|GetTousLesMeublesToutCourt))
  (for _array_element (Variables|TousLesMeubles|GetToutLesMeublesJoueur)
    (Utilities|Array|Add (LocalVariables|GetTousLesMeublesToutCourt) _array_element))
  (for _array_element_2 (Variables|TousLesMeubles|GetTousLesMeublesEnnemis)
    (Utilities|Array|Add (LocalVariables|GetTousLesMeublesToutCourt) _array_element_2))
  (while (Utilities|Array|IsNotEmpty _touslesmeublestoutcourt)
    (LocalVariables|SetCurMaxSpeed -1)
    (LocalVariables|SetCurBestMeuble 0)
    (for _array_element_3 _touslesmeublestoutcourt
      (if (> (Default|GetTrueSpeed _array_element_3) (LocalVariables|GetCurMaxSpeed))
        (LocalVariables|SetCurMaxSpeed (Default|GetTrueSpeed _array_element_3))
        (LocalVariables|SetCurBestMeuble _array_element_3)))
    (Utilities|Array|RemoveItem (LocalVariables|GetTousLesMeublesToutCourt) (LocalVariables|GetCurBestMeuble))
    (Utilities|Array|Add (Variables|TousLesMeubles|GetTousLesMeublesParOrdreDeVitesse) (LocalVariables|GetCurBestMeuble))))

(fn Attaque
  (params (MeubleQuiAttaque :type BP%20Meuble%20Object%20Reference))
  (Default|PlayAnimation MeubleQuiAttaque)
  (LocalVariables|SetEstJoueur (Utilities|Array|ContainsItem (Variables|TousLesMeubles|GetToutLesMeublesJoueur) MeubleQuiAttaque))
  (bind (_cible _effet_de_l_attaque _valeur_principale _valeur_secondaire) (Default|AttaqueGenerale MeubleQuiAttaque))
  (bind _toutlesmeublestouchés (CallFunction|SelectTarget _cible (LocalVariables|GetEstJoueur) (Variables|/Game/Furniture/BP_Meuble.BP_Meuble_C|GetAGaucheEnCombat MeubleQuiAttaque)))
  (CallFunction|DoEffect _effet_de_l_attaque _valeur_principale _valeur_secondaire _toutlesmeublestouchés MeubleQuiAttaque)
  (Default|SetMeublesHealth (Variables|Ref|GetBattleWidgetRef)))

(fn SelectTarget
  (params (Cible :type Enum_CiblesPotentielles%20Enum :default "NewEnumerator0") (Joueur :type Boolean) (PositionGauche :type Boolean))
  (Utilities|Array|Clear (LocalVariables|GetAllTargets))
  (LocalVariables|SetEstJoueur Joueur)
  (LocalVariables|SetAGaucheEnCombat PositionGauche)
  (switch Utilities|FlowControl|Switch|SwitchonEnum_CiblesPotentielles Cible
    (:NewEnumerator0
      (for _array_element (select (LocalVariables|GetEstJoueur) (Variables|TousLesMeubles|GetTousLesMeublesEnnemis) (Variables|TousLesMeubles|GetToutLesMeublesJoueur))
        (if (== (Variables|/Game/Furniture/BP_Meuble.BP_Meuble_C|GetAGaucheEnCombat _array_element) (LocalVariables|GetAGaucheEnCombat))
          (Utilities|Array|Add (LocalVariables|GetAllTargets) _array_element)))
      (if (Utilities|Array|IsEmpty (LocalVariables|GetAllTargets))
        (LocalVariables|SetAllTargets (select (LocalVariables|GetEstJoueur) (Variables|TousLesMeubles|GetTousLesMeublesEnnemis) (Variables|TousLesMeubles|GetToutLesMeublesJoueur))))
      (return (LocalVariables|GetAllTargets)))
    (:NewEnumerator1
      (for _array_element_2 (select (LocalVariables|GetEstJoueur) (Variables|TousLesMeubles|GetTousLesMeublesEnnemis) (Variables|TousLesMeubles|GetToutLesMeublesJoueur))
        (if (!= (Variables|/Game/Furniture/BP_Meuble.BP_Meuble_C|GetAGaucheEnCombat _array_element_2) (LocalVariables|GetAGaucheEnCombat))
          (Utilities|Array|Add (LocalVariables|GetAllTargets) _array_element_2)))
      (if (Utilities|Array|IsEmpty (LocalVariables|GetAllTargets))
        (LocalVariables|SetAllTargets (select (LocalVariables|GetEstJoueur) (Variables|TousLesMeubles|GetTousLesMeublesEnnemis) (Variables|TousLesMeubles|GetToutLesMeublesJoueur))))
      (return (LocalVariables|GetAllTargets)))
    (:NewEnumerator2
      (for _array_element_3 (select (LocalVariables|GetEstJoueur) (Variables|TousLesMeubles|GetToutLesMeublesJoueur) (Variables|TousLesMeubles|GetTousLesMeublesEnnemis))
        (if (!= (Variables|/Game/Furniture/BP_Meuble.BP_Meuble_C|GetAGaucheEnCombat _array_element_3) (LocalVariables|GetAGaucheEnCombat))
          (Utilities|Array|Add (LocalVariables|GetAllTargets) _array_element_3)))
      (return (LocalVariables|GetAllTargets)))
    (:NewEnumerator3
      (for _array_element_4 (select (LocalVariables|GetEstJoueur) (Variables|TousLesMeubles|GetToutLesMeublesJoueur) (Variables|TousLesMeubles|GetTousLesMeublesEnnemis))
        (if (== (Variables|/Game/Furniture/BP_Meuble.BP_Meuble_C|GetAGaucheEnCombat _array_element_4) (LocalVariables|GetAGaucheEnCombat))
          (Utilities|Array|Add (LocalVariables|GetAllTargets) _array_element_4)))
      (return (LocalVariables|GetAllTargets)))
    (:NewEnumerator4
      (LocalVariables|SetAllTargets (select (LocalVariables|GetEstJoueur) (Variables|TousLesMeubles|GetTousLesMeublesEnnemis) (Variables|TousLesMeubles|GetToutLesMeublesJoueur))))
    (:NewEnumerator5
      (LocalVariables|SetAllTargets (select (LocalVariables|GetEstJoueur) (Variables|TousLesMeubles|GetToutLesMeublesJoueur) (Variables|TousLesMeubles|GetTousLesMeublesEnnemis))))
    (:NewEnumerator6
      (LocalVariables|SetAllTargets (select (LocalVariables|GetEstJoueur) (Variables|TousLesMeubles|GetTousLesMeublesEnnemis) (Variables|TousLesMeubles|GetToutLesMeublesJoueur)))
      (for _array_element_5 (select (LocalVariables|GetEstJoueur) (Variables|TousLesMeubles|GetToutLesMeublesJoueur) (Variables|TousLesMeubles|GetTousLesMeublesEnnemis))
        (if (!= (Variables|/Game/Furniture/BP_Meuble.BP_Meuble_C|GetAGaucheEnCombat _array_element_5) (LocalVariables|GetAGaucheEnCombat))
          (Utilities|Array|Add (LocalVariables|GetAllTargets) _array_element_5)))
      (return (LocalVariables|GetAllTargets)))
    (:NewEnumerator7
      (LocalVariables|SetAllTargets (Variables|TousLesMeubles|GetToutLesMeublesJoueur))
      (for _array_element_6 (Variables|TousLesMeubles|GetTousLesMeublesEnnemis)
        (Utilities|Array|Add (LocalVariables|GetAllTargets) _array_element_6))
      (return (LocalVariables|GetAllTargets))))
  (return (LocalVariables|GetAllTargets)))

(fn DoEffect
  (params (Effect :type Enum_SkillEffet%20Enum :default "NewEnumerator0") (ValeurPrincipale :type Integer) (ValeurSecondaire :type Integer) (MeublesTouchés :type Array%20of%20BP%20Meuble%20Object%20References) (MeubleAttaquant :type BP%20Meuble%20Object%20Reference))
  (LocalVariables|SetValue1 ValeurPrincipale)
  (LocalVariables|SetValue2 ValeurSecondaire)
  (LocalVariables|SetTousLesMeublesTouchés MeublesTouchés)
  (LocalVariables|SetAttaquant MeubleAttaquant)
  (switch Utilities|FlowControl|Switch|SwitchonEnum_SkillEffet Effect
    (:NewEnumerator0
      (for _array_element (LocalVariables|GetTousLesMeublesTouchés)
        (Default|TakeDamage _array_element (LocalVariables|GetValue1))))
    (:NewEnumerator1
      (for _array_element_2 (LocalVariables|GetTousLesMeublesTouchés)
        (Default|Heal _array_element_2 (LocalVariables|GetValue1))))
    (:NewEnumerator2
      (for _array_element_3 (LocalVariables|GetTousLesMeublesTouchés)
        (Default|Changement-Attaque _array_element_3 (LocalVariables|GetValue1))))
    (:NewEnumerator4
      (for _array_element_4 (LocalVariables|GetTousLesMeublesTouchés)
        (Default|Changement-Vitesse _array_element_4 (LocalVariables|GetValue1))))
    (:NewEnumerator5
      (for _array_element_5 (LocalVariables|GetTousLesMeublesTouchés)
        (Default|Changement-Attaque _array_element_5 (* (LocalVariables|GetValue1) -1))))
    (:NewEnumerator7
      (for _array_element_6 (LocalVariables|GetTousLesMeublesTouchés)
        (Default|Changement-Vitesse _array_element_6 (* (LocalVariables|GetValue1) -1))))
    (:NewEnumerator8
      (for _array_element_7 (LocalVariables|GetTousLesMeublesTouchés)
        (Default|TakeDamage _array_element_7 (LocalVariables|GetValue1))
        (Default|Changement-Attaque (LocalVariables|GetAttaquant) (* (LocalVariables|GetValue2) -1))))))