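; BP_GooglyEyes is a decor Blueprint that animates googly eyes with randomly timed glances.
; From BeginPlay it randomly picks between looking around, a one-in-three chance, and staring.
; LookAround plays a timeline that slides the static mesh along its relative X axis, then hands off to Stare.
; Stare waits on a short timer before choosing again, forming an endless idle loop.
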(event Custom|LookAround
  (bind _newtrack_0 (Timeline|Timeline PlayFromStart)
    (:Update
      (Transformation|SetRelativeLocation (Variables|Default|GetStaticMesh) (Math|Vector|MakeVector (* _newtrack_0 8.0) 0.0 0.0) false false))
    (:Finished
      (CallFunction|Stare))))

(event Custom|Stare
  (Utilities|Time|SetTimerbyEvent (delegate Custom|ChooseBehaviour) 2.0))

(event Custom|ChooseBehaviour
  (if (== (Math|Random|RandomInteger 3) 0)
    (CallFunction|LookAround)
    (else
      (CallFunction|Stare))))

(event EventBeginPlay
  (CallFunction|ChooseBehaviour))

(fn ConstructionScript)